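; Rifle ammo pickup that adds reserve ammo to the player's rifle.
; On the PickUp input press, it checks through PlayerRef that the rifle is picked up and its MaxAmmo is below the cap.
; It then writes the increased, clamped MaxAmmo into the rifle's ItemInfo struct, plays a 2D pickup sound and destroys itself.
; PlayerRef is not set in this graph, and the BeginPlay, overlap and Tick events are disabled stubs.
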(event `InputAction|PickUp`
  (params (Key :type "Key Structure"))
  (bind _iteminfo (`/Game/Levels/Level_1/Pickups/Weapon_PickUp/BP_MasterWeaponPickUp.ItemInfo` (`/Game/Levels/Level_1/Blueprints/PlayerCharacter/BP_PlayerCharacter.Rifle` (`self.Player_Ref`))))
  (:`Pressed`
    (if (`/Game/Levels/Level_1/Blueprints/PlayerCharacter/BP_PlayerCharacter.IsRiflePicked?` (`self.Player_Ref`))
      (if (< (`.MaxAmmo_8_7F34F914434D618B680E9CBB31D05CBA` (break `/Game/Levels/Level_1/Struct/ItemType` (`/Game/Levels/Level_1/Pickups/Weapon_PickUp/BP_MasterWeaponPickUp.ItemInfo` (`/Game/Levels/Level_1/Blueprints/PlayerCharacter/BP_PlayerCharacter.Rifle` (`self.Player_Ref`))))) 200)
        (setmembers `/Game/Levels/Level_1/Struct/ItemType` :`StructRef` _iteminfo :`MaxAmmo` (`KismetMathLibrary.Clamp` (+ (`.MaxAmmo_8_7F34F914434D618B680E9CBB31D05CBA` (break `/Game/Levels/Level_1/Struct/ItemType` _iteminfo)) 20) 0 200))
        (`GameplayStatics.PlaySound2D` "/Game/MilitaryWeapSilver/Sound/Rifle/Cues/Rifle_AmmoPickup_Cue.Rifle_AmmoPickup_Cue" 1.0 1.0 0.0 null null)
        (`self.K2_DestroyActor`)))))

(fn `UserConstructionScript`
  (`parent.UserConstructionScript`))