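; Base ammo pickup actor that shows a named prompt and highlight when the player is nearby.
; Overlap of its Box by a "Player"-tagged actor shows the widget, passes AmmoName to UI_AmmoPick, enables custom depth on the mesh and enables input.
; Leaving hides both and disables input, though CanPick stays true.
; BeginPlay caches the player character; this graph contains no collection logic.
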(event `self.ReceiveBeginPlay`
  (bind _asbp_player_character (cast `/Game/Levels/Level_1/Blueprints/PlayerCharacter/BP_PlayerCharacter` (`GameplayStatics.GetPlayerCharacter` 0)))
  (set `self.Player_Ref` _asbp_player_character))

(event `self.Box.OnComponentBeginOverlap`
  (params (OverlappedComponent :type "PrimitiveComponent Object Reference") (OtherActor :type "Actor Object Reference") (OtherComp :type "PrimitiveComponent Object Reference") (OtherBodyIndex :type Integer) (bFromSweep :type Boolean) (SweepResult :type "HitResult Structure (by ref)"))
  (if (`self.ActorHasTag` OtherActor "Player")
    (`SceneComponent.SetVisibility` (`self.Widget`) true false)
    (`PrimitiveComponent.SetRenderCustomDepth` (`self.AmmoMesh`) true)
    (bind _asui_ammo_pick (cast `/Game/Levels/Level_1/Blueprints/User_Interface/UI_AmmoPick` (`WidgetComponent.GetUserWidgetObject` (`self.Widget`))))
    (set `/Game/Levels/Level_1/Blueprints/User_Interface/UI_AmmoPick.PickUpName` (`self.AmmoName`) _asui_ammo_pick)
    (set `self.CanPick?` true)
    (`self.EnableInput` (`GameplayStatics.GetPlayerController` 0))))

(event `self.Box.OnComponentEndOverlap`
  (params (OverlappedComponent :type "PrimitiveComponent Object Reference") (OtherActor :type "Actor Object Reference") (OtherComp :type "PrimitiveComponent Object Reference") (OtherBodyIndex :type Integer))
  (if (`self.ActorHasTag` OtherActor "Player")
    (`SceneComponent.SetVisibility` (`self.Widget`) false false)
    (`PrimitiveComponent.SetRenderCustomDepth` (`self.AmmoMesh`) false)
    (set `self.CanPick?` true)
    (`self.DisableInput` (`GameplayStatics.GetPlayerController` 0))))

(fn `UserConstructionScript`)