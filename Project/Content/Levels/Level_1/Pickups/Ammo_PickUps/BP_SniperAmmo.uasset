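; Sniper ammo pickup actor that tops up the player's sniper rifle ammo.
; On the PickUp input, it requires that the player has the sniper and that its MaxAmmo is below the cap.
; It then adds a clamped increment to MaxAmmo in the weapon's ItemInfo struct, plays a pickup sound and destroys itself.
; This graph has no overlap or range check of its own.
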(event `InputAction|PickUp`
  (params (Key :type "Key Structure"))
  (bind _iteminfo (`/Game/Levels/Level_1/Pickups/Weapon_PickUp/BP_MasterWeaponPickUp.ItemInfo` (`/Game/Levels/Level_1/Blueprints/PlayerCharacter/BP_PlayerCharacter.Sniper` (`self.Player_Ref`))))
  (:`Pressed`
    (if (`/Game/Levels/Level_1/Blueprints/PlayerCharacter/BP_PlayerCharacter.IsSniperPicked?` (`self.Player_Ref`))
      (if (< (`.MaxAmmo_8_7F34F914434D618B680E9CBB31D05CBA` (break `/Game/Levels/Level_1/Struct/ItemType` (`/Game/Levels/Level_1/Pickups/Weapon_PickUp/BP_MasterWeaponPickUp.ItemInfo` (`/Game/Levels/Level_1/Blueprints/PlayerCharacter/BP_PlayerCharacter.Sniper` (`self.Player_Ref`))))) 60)
        (setmembers `/Game/Levels/Level_1/Struct/ItemType` :`StructRef` _iteminfo :`MaxAmmo` (`KismetMathLibrary.Clamp` (+ (`.MaxAmmo_8_7F34F914434D618B680E9CBB31D05CBA` (break `/Game/Levels/Level_1/Struct/ItemType` _iteminfo)) 5) 0 60))
        (`GameplayStatics.PlaySound2D` "/Game/MilitaryWeapSilver/Sound/SniperRifle/Cues/SniperRifle_AmmoPickup_Cue.SniperRifle_AmmoPickup_Cue" 1.0 1.0 0.0 null null)
        (`self.K2_DestroyActor`)))))

(fn `UserConstructionScript`
  (`parent.UserConstructionScript`))