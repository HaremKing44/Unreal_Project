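; Master weapon actor that shows a widget and outline on player overlap, passes itself to the player on pickup, and handles firing and reloading.
; Rifles support single, timer-driven burst and gated automatic fire; other weapons fire single shots.
; A camera trace applies randomized damage through BI_TakeDamage and aims muzzle projectiles, which spawn and consume ammo only while aiming down sights.
; Rifle and sniper reloads refill ItemInfo's clip from reserves after a montage delay.
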(event `self.Box.OnComponentBeginOverlap`
  (params (OverlappedComponent :type "PrimitiveComponent Object Reference") (OtherActor :type "Actor Object Reference") (OtherComp :type "PrimitiveComponent Object Reference") (OtherBodyIndex :type Integer) (bFromSweep :type Boolean) (SweepResult :type "HitResult Structure (by ref)"))
  (bind _asbp_player_character (cast `/Game/Levels/Level_1/Blueprints/PlayerCharacter/BP_PlayerCharacter` OtherActor))
  (set `self.PlayerReference` _asbp_player_character)
  (`SceneComponent.SetVisibility` (`self.WeaponWidget`) true false)
  (`PrimitiveComponent.SetRenderCustomDepth` (`self.SkeletalMesh`) true)
  (set `self.CanPick?` true)
  (`self.EnableInput` (`GameplayStatics.GetPlayerController` 0)))

(event `self.Box.OnComponentEndOverlap`
  (params (OverlappedComponent :type "PrimitiveComponent Object Reference") (OtherActor :type "Actor Object Reference") (OtherComp :type "PrimitiveComponent Object Reference") (OtherBodyIndex :type Integer))
  (bind _asbp_player_character (cast `/Game/Levels/Level_1/Blueprints/PlayerCharacter/BP_PlayerCharacter` OtherActor))
  (set `self.PlayerReference` _asbp_player_character)
  (`SceneComponent.SetVisibility` (`self.WeaponWidget`) false false)
  (`PrimitiveComponent.SetRenderCustomDepth` (`self.SkeletalMesh`) false)
  (set `self.CanPick?` false)
  (`self.DisableInput` (`GameplayStatics.GetPlayerController` 0) null))

(event `DestroyBox`
  ;[1 1 1] For AI Weapon
  (`ActorComponent.K2_DestroyComponent` (`self.Box`)))

(event `InputAction|PickUp`
  (params (Key :type "Key Structure"))
  (:`Pressed`
    (if (`self.CanPick?`)
      (`/Game/Levels/Level_1/Blueprints/PlayerCharacter/BP_PlayerCharacter.PickupItem` (`self.PlayerReference`) self)
      (`self.K2_DestroyActor`))))

(event `StartFiring`
  ;[1 1 1] Firing Logic
  (if (>= (`.CurrentAmmo_10_C5E4B5D647967F2015A4F290E9096104` (break `/Game/Levels/Level_1/Struct/ItemType` (`self.ItemInfo`))) 1)
    (if (`self.IsReloading`)
      _
      (elif (`/Game/Levels/Level_1/Blueprints/PlayerCharacter/BP_PlayerCharacter.isSprinting` (`self.PlayerReference`))
        _
        (elif (> (`.CurrentAmmo_10_C5E4B5D647967F2015A4F290E9096104` (break `/Game/Levels/Level_1/Struct/ItemType` (`self.ItemInfo`))) 0)
          (if (`/Game/Levels/Level_1/Blueprints/PlayerCharacter/BP_PlayerCharacter.isRifleEquiped?` (`self.PlayerReference`))
            (switch `/Game/Levels/Level_1/Enum/FireMode` (`self.FireMode`)
              (:`NewEnumerator0`
                (`self.SpawnProjectiles`))
              (:`NewEnumerator1`
                (`self.BurstFiring`))
              (:`NewEnumerator2`
                (`self.FullShot`)))
            (else
              (`self.SpawnProjectiles`))))))
    (else
      (`self.ReloadAmmo`))))

(event `FullShot`
  ;[1 1 1] Automatic Firing Logic
  (`|ExecutionSequence`
    (:`then_0`
      (goto _label :!via `Open`))
    (:`then_1`
      (`/Engine/EditorBlueprintResources/StandardMacros.Gate` true :!label _label
        (:`Exit`
          (`|ExecutionSequence`
            (:`then_0`
              (`KismetSystemLibrary.RetriggerableDelay` 0.15)
              (goto _label))
            (:`then_1`
              (`self.LineTrace`)
              (`self.SpawnProjectiles`))))))))

(event `ToggleFireMode`
  ;[1 1 1] Logic to Change Fire-Mode
  (if (>= (`self.FireModeIndex`) 2)
    (set `self.FireModeIndex` 0)
    (else
      (set `self.FireModeIndex` (+ (`self.FireModeIndex`) 1))))
  (switch `int` (`self.FireModeIndex`)
    (:`0`
      (set `self.FireMode` "NewEnumerator0"))
    (:`1`
      (set `self.FireMode` "NewEnumerator1"))
    (:`2`
      (set `self.FireMode` "NewEnumerator2"))))

(event `ResetFull`
  ;[1 1 1] Automatic Firing Logic
  (goto _label :!via `Close`))

(event `ReloadAmmo`
  (bind ((`MaxAmmo_8_7F34F914434D618B680E9CBB31D05CBA` _maxammo)) (break `/Game/Levels/Level_1/Struct/ItemType` (`self.ItemInfo`)))
  (bind ((`ClipAmmo_25_857405DF4E4DB3B86858EC82260B5FC8` _clipammo) (`CurrentAmmo_10_C5E4B5D647967F2015A4F290E9096104` _currentammo)) (break `/Game/Levels/Level_1/Struct/ItemType` (`self.ItemInfo`)))
  (bind ((`ClipAmmo_25_857405DF4E4DB3B86858EC82260B5FC8` _clipammo_2) (`CurrentAmmo_10_C5E4B5D647967F2015A4F290E9096104` _currentammo_2)) (break `/Game/Levels/Level_1/Struct/ItemType` (`self.ItemInfo`)))
  ;[1 1 1] Reload System Logic
  (if (== (`.MaxAmmo_8_7F34F914434D618B680E9CBB31D05CBA` (break `/Game/Levels/Level_1/Struct/ItemType` (`self.ItemInfo`))) 0)
    (`KismetSystemLibrary.PrintString` "No ammo left")
    (elif (and (or (`/Game/Levels/Level_1/Blueprints/PlayerCharacter/BP_PlayerCharacter.isRifleEquiped?` (`self.PlayerReference`)) (`/Game/Levels/Level_1/Blueprints/PlayerCharacter/BP_PlayerCharacter.isSniperEquiped?` (`self.PlayerReference`))) (!= _clipammo_2 _currentammo_2) (not (`self.IsReloading`)))
      (set `self.IsReloading` true)
      (`Character.PlayAnimMontage` (`self.PlayerReference`) "/Game/Levels/Level_1/Animations/Montages/Reload_Rifle_Hip_Montage.Reload_Rifle_Hip_Montage" 1.0 "None")
      (`KismetSystemLibrary.RetriggerableDelay` 2.0)
      (set `self.Needed Ammos` (- _clipammo _currentammo))
      (if (<= _maxammo (`self.Needed Ammos`))
        (bind _structout (setmembers `/Game/Levels/Level_1/Struct/ItemType` :`StructRef` (`self.ItemInfo`) :`CurrentAmmo` _maxammo))
        (bind ((`MaxAmmo_8_7F34F914434D618B680E9CBB31D05CBA` _maxammo_2) (`CurrentAmmo_10_C5E4B5D647967F2015A4F290E9096104` _currentammo_3)) (break `/Game/Levels/Level_1/Struct/ItemType` _structout))
        (setmembers `/Game/Levels/Level_1/Struct/ItemType` :`StructRef` (`self.ItemInfo`) :`MaxAmmo` (- _maxammo_2 _currentammo_3))
        (else
          (setmembers `/Game/Levels/Level_1/Struct/ItemType` :`StructRef` (`self.ItemInfo`) :`CurrentAmmo` (`.ClipAmmo_25_857405DF4E4DB3B86858EC82260B5FC8` (break `/Game/Levels/Level_1/Struct/ItemType` (`self.ItemInfo`))))
          (setmembers `/Game/Levels/Level_1/Struct/ItemType` :`StructRef` (`self.ItemInfo`) :`MaxAmmo` (- (`.MaxAmmo_8_7F34F914434D618B680E9CBB31D05CBA` (break `/Game/Levels/Level_1/Struct/ItemType` (`self.ItemInfo`))) (`self.Needed Ammos`)))))
      (set `self.IsReloading` false))))

(fn `SpawnProjectiles`
  (bind _playerreference (`self.PlayerReference`))
  (bind _iteminfo (`self.ItemInfo`))
  (bind (_returnvalue_location _returnvalue_rotation _returnvalue_scale) (`KismetMathLibrary.BreakTransform` (`SceneComponent.GetSocketTransform` (`self.SkeletalMesh`) "Muzzle" "RTS_World")))
  (if (>= (`.CurrentAmmo_10_C5E4B5D647967F2015A4F290E9096104` (break `/Game/Levels/Level_1/Struct/ItemType` (`self.ItemInfo`))) 1)
    (`self.LineTrace`)
    (if (`/Game/Levels/Level_1/Blueprints/PlayerCharacter/BP_PlayerCharacter.IsADS?` (`self.PlayerReference`))
      (`|SpawnActorFromClass` "/Game/Levels/Level_1/Blueprints/Projectiles/BP_Projectiles.BP_Projectiles_C" (`self.ProjectileSpawnTransform`) "Undefined" "OverrideRootScale" null null)
      (`GameplayStatics.SpawnEmitterAtLocation` "/Game/FPS_Assault_Pack/Particles/Emitters/Rifle/P_Rifle_Muzzleflash.P_Rifle_Muzzleflash" _returnvalue_location _returnvalue_rotation _returnvalue_scale)
      (setmembers `/Game/Levels/Level_1/Struct/ItemType` :`StructRef` _iteminfo :`CurrentAmmo` (- (`.CurrentAmmo_10_C5E4B5D647967F2015A4F290E9096104` (break `/Game/Levels/Level_1/Struct/ItemType` _iteminfo)) 1))
      (if (`/Game/Levels/Level_1/Blueprints/PlayerCharacter/BP_PlayerCharacter.IsADS?` _playerreference)
        (`Character.PlayAnimMontage` _playerreference "/Game/Levels/Level_1/Animations/Montages/Fire_Rifle_Ironsights_Montage.Fire_Rifle_Ironsights_Montage" 1.0 "None")))
    (else
      ;[1 1 1] For fullauto Firemode
      (`self.ReloadAmmo`))))

(fn `UserConstructionScript`
  (bind (_iteminfo_itemtype _iteminfo_itemclass _iteminfo_clipammo _iteminfo_maxammo _iteminfo_currentammo _iteminfo_damage _iteminfo_itemimage _iteminfo_equipsocketname _iteminfo_unequipsocketname) (break `/Game/Levels/Level_1/Struct/ItemType` (`self.ItemInfo`)))
  (set `self.ItemInfo` (make `/Game/Levels/Level_1/Struct/ItemType` _iteminfo_itemtype (`GameplayStatics.GetObjectClass` self) _iteminfo_clipammo _iteminfo_maxammo _iteminfo_currentammo _iteminfo_damage _iteminfo_itemimage _iteminfo_equipsocketname _iteminfo_unequipsocketname)))