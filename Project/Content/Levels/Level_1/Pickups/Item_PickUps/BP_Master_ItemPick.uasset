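; Base pickup actor for health packs and keys that the player collects with the PickUp input.
; Box overlap with a Player-tagged actor toggles the name widget, the mesh's custom-depth rendering, the CanPick flag and input handling.
; Pressing PickUp while CanPick is set increments the matching HealthPack or Key count on BP_PlayerCharacter, chosen by PickItemType, then destroys the item.
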(event `self.ReceiveBeginPlay`
  (bind _asui_pick_up_item (cast `/Game/Levels/Level_1/Blueprints/User_Interface/UI_PickUPItem` (`WidgetComponent.GetUserWidgetObject` (`self.Widget`))))
  (set `/Game/Levels/Level_1/Blueprints/User_Interface/UI_PickUPItem.PickUpItemName` (`self.ItemName`) _asui_pick_up_item)
  (bind _asbp_player_character (cast `/Game/Levels/Level_1/Blueprints/PlayerCharacter/BP_PlayerCharacter` (`GameplayStatics.GetPlayerCharacter` 0)))
  (set `self.Player_Ref` _asbp_player_character))

(event `self.Box.OnComponentBeginOverlap`
  (params (OverlappedComponent :type "PrimitiveComponent Object Reference") (OtherActor :type "Actor Object Reference") (OtherComp :type "PrimitiveComponent Object Reference") (OtherBodyIndex :type Integer) (bFromSweep :type Boolean) (SweepResult :type "HitResult Structure (by ref)"))
  (if (`self.ActorHasTag` OtherActor "Player")
    (`SceneComponent.SetVisibility` (`self.Widget`) true false)
    (`PrimitiveComponent.SetRenderCustomDepth` (`self.StaticMesh`) true)
    (set `self.CanPick?` true)
    (`self.EnableInput` (`GameplayStatics.GetPlayerController` 0))))

(event `self.Box.OnComponentEndOverlap`
  (params (OverlappedComponent :type "PrimitiveComponent Object Reference") (OtherActor :type "Actor Object Reference") (OtherComp :type "PrimitiveComponent Object Reference") (OtherBodyIndex :type Integer))
  (if (`self.ActorHasTag` OtherActor "Player")
    (`SceneComponent.SetVisibility` (`self.Widget`) false false)
    (`PrimitiveComponent.SetRenderCustomDepth` (`self.StaticMesh`) false)
    (set `self.CanPick?` false)
    (`self.DisableInput` (`GameplayStatics.GetPlayerController` 0) null)))

(event `InputAction|PickUp`
  (params (Key :type "Key Structure"))
  (bind _player_ref (`self.Player_Ref`))
  (:`Pressed`
    (if (`self.CanPick?`)
      (switch `/Game/Levels/Level_1/Enum/PickUpType` (`self.PickItemType`)
        (:`NewEnumerator1`
          (bind _result (`/Engine/EditorBlueprintResources/StandardMacros.IncrementInt` (`/Game/Levels/Level_1/Blueprints/PlayerCharacter/BP_PlayerCharacter.HealthPack` _player_ref))
            (:`  `
              (set `/Game/Levels/Level_1/Blueprints/PlayerCharacter/BP_PlayerCharacter.HealthPack` _result _player_ref)
              (`self.K2_DestroyActor`))))
        (:`NewEnumerator2`
          (bind _result_2 (`/Engine/EditorBlueprintResources/StandardMacros.IncrementInt` (`/Game/Levels/Level_1/Blueprints/PlayerCharacter/BP_PlayerCharacter.Key` _player_ref))
            (:`  `
              (set `/Game/Levels/Level_1/Blueprints/PlayerCharacter/BP_PlayerCharacter.Key` _result_2 _player_ref)
              (`self.K2_DestroyActor`))))))))

(fn `UserConstructionScript`)