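; Level 1 door Blueprint that swings open for a player holding at least one key, unless it is flagged as jammed.
; BeginPlay caches the player character and sets the door widget's text to either the jam message or a key hint.
; Box overlap by a "Player"-tagged actor toggles the widget; entering with a key clears the text and plays a timeline rotating the mesh's yaw.
; The key count is not decremented.
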(event `self.ReceiveBeginPlay`
  (bind _asbp_player_character (cast `/Game/Levels/Level_1/Blueprints/PlayerCharacter/BP_PlayerCharacter` (`GameplayStatics.GetPlayerCharacter` 0)))
  (set `self.PlayerRef` _asbp_player_character)
  (bind _asui_door (cast `/Game/Levels/Level_1/Blueprints/User_Interface/UI_Door` (`WidgetComponent.GetUserWidgetObject` (`self.JDoorWidget`))))
  (if (`self.IsJammed`)
    (set `/Game/Levels/Level_1/Blueprints/User_Interface/UI_Door.DoorMessage` (`self.JamMsg`) _asui_door)
    (elif true
      (set `/Game/Levels/Level_1/Blueprints/User_Interface/UI_Door.DoorMessage` "FIND A KEY TO OPEN THIS DOOR!" _asui_door))))

(event `self.Box.OnComponentBeginOverlap`
  (params (OverlappedComponent :type "PrimitiveComponent Object Reference") (OtherActor :type "Actor Object Reference") (OtherComp :type "PrimitiveComponent Object Reference") (OtherBodyIndex :type Integer) (bFromSweep :type Boolean) (SweepResult :type "HitResult Structure (by ref)"))
  (if (`self.ActorHasTag` OtherActor "Player")
    (`SceneComponent.SetVisibility` (`self.JDoorWidget`) true false)
    (if (not (`self.IsJammed`))
      (if (> (`/Game/Levels/Level_1/Blueprints/PlayerCharacter/BP_PlayerCharacter.Key` (`self.PlayerRef`)) 0)
        (set `/Game/Levels/Level_1/Blueprints/User_Interface/UI_Door.DoorMessage` "" (stale `self.ReceiveBeginPlay` _asui_door))
        (bind (_direction _zangle) (`Timeline|OpenDoor`)
          (:`Update`
            (`SceneComponent.K2_SetRelativeRotation` (`self.SM_Door`) (`KismetMathLibrary.MakeRotator` 0.0 0.0 _zangle) false false)))))))

(event `self.Box.OnComponentEndOverlap`
  (params (OverlappedComponent :type "PrimitiveComponent Object Reference") (OtherActor :type "Actor Object Reference") (OtherComp :type "PrimitiveComponent Object Reference") (OtherBodyIndex :type Integer))
  (if (`self.ActorHasTag` OtherActor "Player")
    (`SceneComponent.SetVisibility` (`self.JDoorWidget`) false false)))

(fn `UserConstructionScript`)