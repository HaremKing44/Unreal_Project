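; BP_WeaponEquip is a weapon pickup that offers its weapon to the player standing inside its Box trigger.
; On begin overlap it casts to BP_PlayerCharacter, stores the reference, shows WeaponWidget and sets the player's AttachedWeapon to WeaponToAdd.
; End overlap hides the widget and clears AttachedWeapon on the stored player, without checking which actor left.
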(event `self.Box.OnComponentBeginOverlap`
  (params (OverlappedComponent :type "PrimitiveComponent Object Reference") (OtherActor :type "Actor Object Reference") (OtherComp :type "PrimitiveComponent Object Reference") (OtherBodyIndex :type Integer) (bFromSweep :type Boolean) (SweepResult :type "HitResult Structure (by ref)"))
  (bind _asbp_player_character (cast `/Game/Levels/Level_1/Blueprints/PlayerCharacter/BP_PlayerCharacter` OtherActor))
  (set `self.PlayerReference` _asbp_player_character)
  (if true
    (`SceneComponent.SetVisibility` (`self.WeaponWidget`) true false)
    (set `/Game/Levels/Level_1/Blueprints/PlayerCharacter/BP_PlayerCharacter.AttachedWeapon` (`self.WeaponToAdd`) (`self.PlayerReference`))))

(event `self.Box.OnComponentEndOverlap`
  (params (OverlappedComponent :type "PrimitiveComponent Object Reference") (OtherActor :type "Actor Object Reference") (OtherComp :type "PrimitiveComponent Object Reference") (OtherBodyIndex :type Integer))
  (if true
    (`SceneComponent.SetVisibility` (`self.WeaponWidget`) false false)
    (set `/Game/Levels/Level_1/Blueprints/PlayerCharacter/BP_PlayerCharacter.AttachedWeapon` null (`self.PlayerReference`))))

(fn `UserConstructionScript`)