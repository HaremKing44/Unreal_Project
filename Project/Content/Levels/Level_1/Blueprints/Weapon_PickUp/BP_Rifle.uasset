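; BP_Rifle is the player's rifle weapon, with single, burst and full-auto fire modes cycled by input.
; Firing requires the rifle equipped and no sprint or reload, then spawns muzzle projectiles using a looping timer for burst and auto.
; A camera line trace runs on firing, but its result is unused.
; Reloading plays a montage, waits, then refills the clip from reserve ammo in ItemInfo, also triggering when empty.
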(event `self.ReceiveBeginPlay`
  (`self.GetPlayerReference`))

(event `InputAction|FireMode`
  (params (Key :type "Key Structure"))
  ;[1 1 1] Logic to change Fire Mode
  (:`Pressed`
    (if (>= (`self.FireModeIndex`) 2)
      (set `self.FireModeIndex` 0)
      (else
        (set `self.FireModeIndex` (+ (`self.FireModeIndex`) 1))))
    (switch `int` (`self.FireModeIndex`)
      (:`0`
        (set `self.FireMode` "NewEnumerator0"))
      (:`1`
        (set `self.FireMode` "NewEnumerator1"))
      (:`2`
        (set `self.FireMode` "NewEnumerator2")))))

(event `StartFiring`
  (bind _camera (`/Game/Levels/Level_1/Blueprints/PlayerCharacter/BP_PlayerCharacter.Camera` (`self.Player_Reference`)))
  (bind _returnvalue (`SceneComponent.K2_GetComponentLocation` _camera))
  ;[1 1 1] Fire projectile
  (if (`self.isReloading`)
    _
    (elif (`/Game/Levels/Level_1/Blueprints/PlayerCharacter/BP_PlayerCharacter.isSprinting` (`self.Player_Reference`))
      _
      (elif (`/Game/Levels/Level_1/Blueprints/PlayerCharacter/BP_PlayerCharacter.isRifleEquiped?` (`self.Player_Reference`))
        (if (> (`.CurrentAmmo_10_C5E4B5D647967F2015A4F290E9096104` (break `/Game/Levels/Level_1/Struct/ItemType` (`self.ItemInfo`))) 0)
          (`KismetSystemLibrary.LineTraceSingle` _returnvalue (+ _returnvalue (* (`KismetMathLibrary.GetForwardVector` (`SceneComponent.K2_GetComponentRotation` _camera)) 15000)) "TraceTypeQuery1")
          (switch `/Game/Levels/Level_1/Enum/FireMode` (`self.FireMode`)
            (:`NewEnumerator0`
              (`self.SpawnProjectiles`))
            (:`NewEnumerator1`
              (`self.BurstShot`))
            (:`NewEnumerator2`
              (bind _returnvalue_2 (`KismetSystemLibrary.K2_SetTimer` null "SpawnProjectiles" 0.1 true))
              (set `self.FullShotTimer` _returnvalue_2))))))))

(event `StopFiring`
  ;[1 1 1] Fire projectile
  (if (`KismetSystemLibrary.K2_IsValidTimerHandle` (`self.FullShotTimer`))
    (`KismetSystemLibrary.K2_ClearTimer` null "SpawnProjectiles")))

(event `InputAction|Reload`
  (params (Key :type "Key Structure"))
  ;[1 1 1] Reload Input
  (:`Pressed`
    (`self.ReloadAmmo`)))

(event `InputAction|Fire`
  (params (Key :type "Key Structure"))
  ;[1 1 1] Fire Input
  (:`Pressed`
    (if (>= (`.CurrentAmmo_10_C5E4B5D647967F2015A4F290E9096104` (break `/Game/Levels/Level_1/Struct/ItemType` (`self.ItemInfo`))) 1)
      (`self.StartFiring`)
      (else
        (`self.ReloadAmmo`))))
  (:`Released`
    (`self.StopFiring`)))

(event `ReloadAmmo`
  (bind ((`MaxAmmo_8_7F34F914434D618B680E9CBB31D05CBA` _maxammo)) (break `/Game/Levels/Level_1/Struct/ItemType` (`self.ItemInfo`)))
  (bind ((`ClipAmmo_25_857405DF4E4DB3B86858EC82260B5FC8` _clipammo) (`CurrentAmmo_10_C5E4B5D647967F2015A4F290E9096104` _currentammo)) (break `/Game/Levels/Level_1/Struct/ItemType` (`self.ItemInfo`)))
  (bind ((`ClipAmmo_25_857405DF4E4DB3B86858EC82260B5FC8` _clipammo_2) (`CurrentAmmo_10_C5E4B5D647967F2015A4F290E9096104` _currentammo_2)) (break `/Game/Levels/Level_1/Struct/ItemType` (`self.ItemInfo`)))
  ;[1 1 1] Reloading System
  (if (== (`.MaxAmmo_8_7F34F914434D618B680E9CBB31D05CBA` (break `/Game/Levels/Level_1/Struct/ItemType` (`self.ItemInfo`))) 0)
    (`KismetSystemLibrary.PrintString` "No ammo left")
    (elif (and (`/Game/Levels/Level_1/Blueprints/PlayerCharacter/BP_PlayerCharacter.isRifleEquiped?` (`self.Player_Reference`)) (!= _clipammo_2 _currentammo_2) (not (`self.isReloading`)))
      (set `self.isReloading` true)
      (`Character.PlayAnimMontage` (`self.Player_Reference`) "/Game/Levels/Level_1/Animations/Montages/Reload_Rifle_Hip_Montage.Reload_Rifle_Hip_Montage" 1.0 "None")
      (`KismetSystemLibrary.RetriggerableDelay` 2.0)
      (set `self.NeededAmmos` (- _clipammo _currentammo))
      (if (<= _maxammo (`self.NeededAmmos`))
        (bind _structout (setmembers `/Game/Levels/Level_1/Struct/ItemType` :`StructRef` (`self.ItemInfo`) :`CurrentAmmo` _maxammo))
        (bind ((`MaxAmmo_8_7F34F914434D618B680E9CBB31D05CBA` _maxammo_2) (`CurrentAmmo_10_C5E4B5D647967F2015A4F290E9096104` _currentammo_3)) (break `/Game/Levels/Level_1/Struct/ItemType` _structout))
        (setmembers `/Game/Levels/Level_1/Struct/ItemType` :`StructRef` (`self.ItemInfo`) :`MaxAmmo` (- _maxammo_2 _currentammo_3))
        (else
          (setmembers `/Game/Levels/Level_1/Struct/ItemType` :`StructRef` (`self.ItemInfo`) :`CurrentAmmo` (`.ClipAmmo_25_857405DF4E4DB3B86858EC82260B5FC8` (break `/Game/Levels/Level_1/Struct/ItemType` (`self.ItemInfo`))))
          (setmembers `/Game/Levels/Level_1/Struct/ItemType` :`StructRef` (`self.ItemInfo`) :`MaxAmmo` (- (`.MaxAmmo_8_7F34F914434D618B680E9CBB31D05CBA` (break `/Game/Levels/Level_1/Struct/ItemType` (`self.ItemInfo`))) (`self.NeededAmmos`)))))
      (set `self.isReloading` false))))

(fn `SpawnProjectiles`
  (bind _iteminfo (`self.ItemInfo`))
  (if (>= (`.CurrentAmmo_10_C5E4B5D647967F2015A4F290E9096104` (break `/Game/Levels/Level_1/Struct/ItemType` (`self.ItemInfo`))) 1)
    (`|SpawnActorFromClass` (`self.Projectiles`) (`SceneComponent.K2_GetComponentToWorld` (`self.MuzzlePoint`)) "Undefined" "OverrideRootScale" null null)
    (setmembers `/Game/Levels/Level_1/Struct/ItemType` :`StructRef` _iteminfo :`CurrentAmmo` (- (`.CurrentAmmo_10_C5E4B5D647967F2015A4F290E9096104` (break `/Game/Levels/Level_1/Struct/ItemType` _iteminfo)) 1))
    (else
      ;[1 1 1] For fullauto Firemode
      (`self.ReloadAmmo`))))

(fn `UserConstructionScript`
  (`parent.UserConstructionScript`))