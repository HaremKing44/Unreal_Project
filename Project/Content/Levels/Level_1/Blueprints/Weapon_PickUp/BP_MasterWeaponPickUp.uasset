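; Master weapon pickup actor that lets the player collect a weapon when standing near it.
; Box overlap with BP_PlayerCharacter toggles the prompt widget, custom-depth mesh highlight and CanPick flag, enabling input on entry and calling DisableInput on exit.
; Pressing PickUp passes the actor to the player's PickupItem, then destroys it.
; The construction script writes the actor's own class into ItemInfo, keeping the other item fields.
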(event `self.Box.OnComponentBeginOverlap`
  (params (OverlappedComponent :type "PrimitiveComponent Object Reference") (OtherActor :type "Actor Object Reference") (OtherComp :type "PrimitiveComponent Object Reference") (OtherBodyIndex :type Integer) (bFromSweep :type Boolean) (SweepResult :type "HitResult Structure (by ref)"))
  (bind _asbp_player_character (cast `/Game/Levels/Level_1/Blueprints/PlayerCharacter/BP_PlayerCharacter` OtherActor))
  (set `self.PlayerReference` _asbp_player_character)
  (`SceneComponent.SetVisibility` (`self.WeaponWidget`) true false)
  (`PrimitiveComponent.SetRenderCustomDepth` (`self.SkeletalMesh`) true)
  (set `self.CanPick?` true)
  (`self.EnableInput` (`GameplayStatics.GetPlayerController` 0)))

(event `self.Box.OnComponentEndOverlap`
  (params (OverlappedComponent :type "PrimitiveComponent Object Reference") (OtherActor :type "Actor Object Reference") (OtherComp :type "PrimitiveComponent Object Reference") (OtherBodyIndex :type Integer))
  (bind _asbp_player_character (cast `/Game/Levels/Level_1/Blueprints/PlayerCharacter/BP_PlayerCharacter` OtherActor))
  (set `self.PlayerReference` _asbp_player_character)
  (`SceneComponent.SetVisibility` (`self.WeaponWidget`) false false)
  (`PrimitiveComponent.SetRenderCustomDepth` (`self.SkeletalMesh`) false)
  (set `self.CanPick?` false)
  (`self.DisableInput` (`GameplayStatics.GetPlayerController` 0) null))

(event `InputAction|PickUp`
  (params (Key :type "Key Structure"))
  (:`Pressed`
    (if (`self.CanPick?`)
      (`/Game/Levels/Level_1/Blueprints/PlayerCharacter/BP_PlayerCharacter.PickupItem` (`self.PlayerReference`) self)
      (`self.K2_DestroyActor`))))

(fn `UserConstructionScript`
  (bind (_iteminfo_itemtype _iteminfo_itemclass _iteminfo_maxammo _iteminfo_currentammo _iteminfo_damage _iteminfo_itemimage _iteminfo_equipsocketname _iteminfo_unequipsocketname) (break `/Game/Levels/Level_1/Struct/ItemType` (`self.ItemInfo`)))
  (set `self.ItemInfo` (make `/Game/Levels/Level_1/Struct/ItemType` _iteminfo_itemtype (`GameplayStatics.GetObjectClass` self) _iteminfo_maxammo _iteminfo_currentammo _iteminfo_damage _iteminfo_itemimage _iteminfo_equipsocketname _iteminfo_unequipsocketname)))