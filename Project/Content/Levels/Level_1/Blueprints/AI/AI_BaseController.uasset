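; AI controller for BP_Master_AI enemies that patrol a spline path and hunt the player.
; Patrol ping-pongs between spline points with pauses, while a looping timer polls combat state.
; A found enemy triggers combat and pursuit into firing range; player death returns to patrol, and AI death halts the controller.
; Firing uses a muzzle line trace, applying interface damage and spawning a projectile toward the impact on a hit.
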(event `self.ReceiveBeginPlay`
  (bind _asbp_master_ai (cast `/Game/Levels/Level_1/Blueprints/AI/BP_Master_AI` (`self.K2_GetPawn`)))
  (set `self.AI_Ref` _asbp_master_ai)
  (bind _returnvalue (`KismetSystemLibrary.K2_SetTimer` null "Check" 0.4 true))
  (set `self.Clear Timer` _returnvalue)
  (`self.Patrolling`))

(event `Check`
  (if (`/Game/Levels/Level_1/Blueprints/PlayerCharacter/BP_PlayerCharacter.IsDead?` (cast `/Game/Levels/Level_1/Blueprints/PlayerCharacter/BP_PlayerCharacter` (`GameplayStatics.GetPlayerCharacter` 0) :!pure true))
    (`/Engine/EditorBlueprintResources/StandardMacros.DoOnce` false
      (:`Completed`
        (`/Game/Levels/Level_1/Blueprints/AI/BP_Master_AI.EnableCombat` (`self.AI_Ref`))
        (`KismetSystemLibrary.Delay` 2.0)
        (`self.Patrolling`)))
    (elif (not (`/Game/Levels/Level_1/Blueprints/AI/BP_Master_AI.IsDead?` (`self.AI_Ref`)))
      (if (`/Game/Levels/Level_1/Blueprints/AI/BP_Master_AI.IsEnemyFound?` (`self.AI_Ref`))
        (`|ExecutionSequence`
          (:`then_0`
            (`self.HuntEnemy`))
          (:`then_1`
            (`/Engine/EditorBlueprintResources/StandardMacros.DoOnce` false
              (:`Completed`
                (`/Game/Levels/Level_1/Blueprints/AI/BP_Master_AI.EnableCombat` (`self.AI_Ref`)))))))
      (else
        (`KismetSystemLibrary.K2_ClearAndInvalidateTimerHandle` (`self.Clear Timer`))
        (`self.StopMovement`)))))

(event `Patrolling`
  (bind _ai_ref (`self.AI_Ref`))
  (bind _ai_ref_2 (`self.AI_Ref`))
  (bind _splineindex (`/Game/Levels/Level_1/Blueprints/AI/BP_Master_AI.SplineIndex` _ai_ref_2))
  (bind _splineindex_2 (`/Game/Levels/Level_1/Blueprints/AI/BP_Master_AI.SplineIndex` _ai_ref))
  (if (not (`/Game/Levels/Level_1/Blueprints/AI/BP_Master_AI.IsEnemyFound?` (`self.AI_Ref`)))
    (if (`self.WalkBack?`)
      (`|AIMoveTo` _ai_ref_2 (`SplineComponent.GetLocationAtSplinePoint` (`/Game/Levels/Level_1/Blueprints/AI/BP_Master_AI.Path` _ai_ref_2) _splineindex "World") null
        (:`OnSuccess`
          (if (== _splineindex 0)
            (set `self.WalkBack?` false)
            (else
              (`/Engine/EditorBlueprintResources/StandardMacros.DecrementInt` (`/Game/Levels/Level_1/Blueprints/AI/BP_Master_AI.SplineIndex` (`self.AI_Ref`))
                (:`  `
                  _))))
          (`KismetSystemLibrary.Delay` 4.0)
          (`self.Patrolling`)))
      (else
        (`|AIMoveTo` _ai_ref (`SplineComponent.GetLocationAtSplinePoint` (`/Game/Levels/Level_1/Blueprints/AI/BP_Master_AI.Path` _ai_ref) _splineindex_2 "World") null
          (:`OnSuccess`
            (if (== _splineindex_2 (`/Game/Levels/Level_1/Blueprints/AI/BP_Master_AI.MaxPathPoint` _ai_ref))
              (set `self.WalkBack?` true)
              (else
                (`/Engine/EditorBlueprintResources/StandardMacros.IncrementInt` (`/Game/Levels/Level_1/Blueprints/AI/BP_Master_AI.SplineIndex` (`self.AI_Ref`))
                  (:`  `
                    _))))
            (`KismetSystemLibrary.Delay` 4.0)
            (`self.Patrolling`)))))))

(event `HuntEnemy`
  (`|AIMoveTo` (`self.AI_Ref`) (0.0 0.0 0.0) (`GameplayStatics.GetPlayerCharacter` 0) 1000.0
    (:`OnSuccess`
      (`self.AI_FireAmmo`))))

(event `AI_FireAmmo`
  (bind _skeletalmesh (`/Game/Levels/Level_1/Blueprints/Weapon_PickUp/BP_MasterWeaponPickUp.SkeletalMesh` (`/Game/Levels/Level_1/Blueprints/AI/BP_Master_AI.AI_WeaponRef` (`self.AI_Ref`))))
  (bind _returnvalue (`SceneComponent.GetSocketLocation` _skeletalmesh "Muzzle"))
  (bind _returnvalue_2 (`SceneComponent.GetSocketLocation` (`/Game/Levels/Level_1/Blueprints/Weapon_PickUp/BP_MasterWeaponPickUp.SkeletalMesh` (`/Game/Levels/Level_1/Blueprints/AI/BP_Master_AI.AI_WeaponRef` (`self.AI_Ref`))) "Muzzle"))
  (bind (_outhit _returnvalue_3) (`KismetSystemLibrary.LineTraceSingle` _returnvalue (+ _returnvalue (* (`KismetMathLibrary.GreaterGreater_VectorRotator` (`SceneComponent.GetForwardVector` _skeletalmesh) (struct :`Yaw` 93.0)) 15000)) "TraceTypeQuery1"))
  (if _returnvalue_3
    (bind (_bblockinghit _binitialoverlap _time _distance _location _impactpoint _normal _impactnormal _physmat _hitactor _hitcomponent _hitbonename _hititem _faceindex _tracestart _traceend) (`GameplayStatics.BreakHitResult` _outhit))
    (if (`KismetSystemLibrary.DoesImplementInterface` _hitactor "/Game/Levels/BI_TakeDamage.BI_TakeDamage_C")
      (message `/Game/Levels/BI_TakeDamage.ITakeDamage` _hitactor _hitbonename 20.0))
    (`|SpawnActorFromClass` "/Game/Levels/Level_1/Blueprints/Projectiles/BP_Projectiles.BP_Projectiles_C" (`KismetMathLibrary.MakeTransform` _returnvalue_2 (`KismetMathLibrary.FindLookAtRotation` _returnvalue_2 (`KismetMathLibrary.SelectVector` _impactpoint _traceend _returnvalue_3))) "Undefined" "OverrideRootScale" null null)))

(fn `UserConstructionScript`)