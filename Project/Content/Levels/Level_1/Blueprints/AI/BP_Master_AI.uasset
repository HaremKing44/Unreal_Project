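; Master AI character with health, a holstered weapon, an overhead-style state widget and a spline path.
; On BeginPlay it links the UI_AIState widget to itself and spawns its weapon on the back socket; EnableCombat plays the equip montage, while a separate FlipFlop event swaps sockets and combat flags.
; Interface damage makes headshots lethal and other hits alert it; death triggers ragdoll.
; Construction detaches the path in world space and caches its point count.
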(event `self.ReceiveBeginPlay`
  (set `self.CurrentHealth` (`self.MaxHealth`))
  (bind _asui_aistate (cast `/Game/Levels/Level_1/Blueprints/User_Interface/UI_AIState` (`WidgetComponent.GetUserWidgetObject` (`self.AI_Widget`))))
  (set `/Game/Levels/Level_1/Blueprints/User_Interface/UI_AIState.Owner` self _asui_aistate)
  (`self.SpawnWeapon`))

(event `/Game/Levels/BI_TakeDamage.ITakeDamage`
  (params (BoneName :type Name) (Damage :type "Float (single-precision)"))
  ;[1 1 1] Damage Function by using Blueprint Interface
  (if (== BoneName "Head")
    (set `self.CurrentHealth` 0.0)
    (set `self.IsDead?` true :!label _label)
    (`SkeletalMeshComponent.SetAllBodiesSimulatePhysics` (`self.Mesh`) true)
    (`PrimitiveComponent.SetCollisionEnabled` (`self.CapsuleComponent`) "NoCollision")
    (`SceneComponent.SetVisibility` (`self.AI_Widget`) false false)
    (else
      (set `self.IsEnemyFound?` true)
      (set `self.CurrentHealth` (- (`self.CurrentHealth`) Damage))
      (if (<= (`self.CurrentHealth`) 0.0)
        (goto _label)))))

(event `Equip/UnEquip`
  (`/Engine/EditorBlueprintResources/StandardMacros.FlipFlop`
    (:`A`
      (`self.K2_AttachToComponent` (`self.AI_WeaponRef`) (`self.Mesh`) "GunSocket" "SnapToTarget" "SnapToTarget" "SnapToTarget" true)
      (set `self.WeaponEquiped?` true))
    (:`B`
      (`self.K2_AttachToComponent` (`self.AI_WeaponRef`) (`self.Mesh`) "BackGunSocket" "SnapToTarget" "SnapToTarget" "SnapToTarget" true)
      (set `self.WeaponEquiped?` false)
      (set `self.IsEnemyFound?` false))))

(event `SpawnWeapon`
  (bind _returnvalue (`|SpawnActorFromClass` (`self.EquipWeaponClass`) (`SceneComponent.K2_GetComponentToWorld` (`self.Sphere`)) "Undefined" "OverrideRootScale" null null))
  (bind _output_get (set `self.AI_WeaponRef` _returnvalue))
  (`self.K2_AttachToComponent` _output_get (`self.Mesh`) "BackGunSocket" "SnapToTarget" "SnapToTarget" "SnapToTarget" true)
  (`/Game/Levels/Level_1/Blueprints/Weapon_PickUp/BP_MasterWeaponPickUp.DestroyBox` (`self.AI_WeaponRef`)))

(event `EnableCombat`
  (`self.PlayAnimMontage` "/Game/Levels/Level_1/Animations/Montages/Equip_Rifle_Standing_Montage.Equip_Rifle_Standing_Montage"))

(fn `UserConstructionScript`
  (bind _path (`self.Path`))
  (`SceneComponent.K2_DetachFromComponent` _path "KeepWorld" "KeepWorld" "KeepWorld" true)
  (set `self.MaxPathPoint` (`SplineComponent.GetNumberOfSplinePoints` _path)))