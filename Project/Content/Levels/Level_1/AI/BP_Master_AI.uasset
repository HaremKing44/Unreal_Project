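; Base enemy AI character that spawns a weapon, detects the player and alerts to fellow AI.
; Pawn sensing, non-fatal damage and an alert-area overlap with alerted or dead allies set IsEnemyFound, with corpses investigated first.
; Interface damage makes headshots instantly lethal, and death triggers ragdoll.
; Helper events toggle the weapon between hand and back, line-trace for sight and yaw the state widget toward the player; construction detaches the path spline.
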(event `Rotate_AIWidget`
  (bind _returnvalue (`GameplayStatics.GetPlayerCharacter` 0))
  (bind (_returnvalue_roll _returnvalue_pitch _returnvalue_yaw) (`KismetMathLibrary.BreakRotator` (`KismetMathLibrary.FindLookAtRotation` (`SceneComponent.K2_GetComponentLocation` (`self.AI_Widget`)) (`SceneComponent.K2_GetComponentLocation` (`Character.Mesh` _returnvalue)))))
  ;[1 1 1] Rotate AI Widget toward Player
  (if (`self.ActorHasTag` _returnvalue "Player")
    (`SceneComponent.K2_SetWorldRotation` (`self.AI_Widget`) (`KismetMathLibrary.MakeRotator` 0.0 0.0 _returnvalue_yaw) false false)))

(event `self.ReceiveBeginPlay`
  (set `self.CurrentHealth` (`self.MaxHealth`))
  (bind _asui_aistate (cast `/Game/Levels/Level_1/Blueprints/User_Interface/UI_AIState` (`WidgetComponent.GetUserWidgetObject` (`self.AI_Widget`))))
  (set `/Game/Levels/Level_1/Blueprints/User_Interface/UI_AIState.Owner` self _asui_aistate)
  (`self.SpawnWeapon`))

(event `/Game/Levels/Level_1/Blueprints/Blueprint_Interface/BI_TakeDamage.ITakeDamage`
  (params (BoneName :type Name) (Damage :type "Float (single-precision)"))
  ;[1 1 1] Damage Function by using Blueprint Interface
  (if (== BoneName "Head")
    (set `self.CurrentHealth` 0.0)
    (`/Engine/EditorBlueprintResources/StandardMacros.DoOnce` false :!label _label
      (:`Completed`
        (set `self.IsDead?` true)
        (`SkeletalMeshComponent.SetAllBodiesSimulatePhysics` (`self.Mesh`) true)
        (`PrimitiveComponent.SetCollisionEnabled` (`self.CapsuleComponent`) "NoCollision")
        (`SceneComponent.SetVisibility` (`self.AI_Widget`) false false)
        (`ActorComponent.K2_DestroyComponent` (`self.AlertArea`))))
    (else
      (set `self.IsEnemyFound?` true)
      (set `self.CurrentHealth` (- (`self.CurrentHealth`) Damage))
      (if (<= (`self.CurrentHealth`) 0.0)
        (goto _label)))))

(event `EnableCombat`
  ;[1 1 1] Equip/Unequip Weapon
  (`self.PlayAnimMontage` "/Game/Levels/Level_1/Animations/Montages/Equip_Rifle_Standing_Montage.Equip_Rifle_Standing_Montage" 2.0))

(event `Equip/UnEquip`
  ;[1 1 1] Equip/Unequip Weapon
  (`/Engine/EditorBlueprintResources/StandardMacros.FlipFlop`
    (:`A`
      (`self.K2_AttachToComponent` (`self.AI_WeaponRef`) (`self.Mesh`) "GunSocket" "SnapToTarget" "SnapToTarget" "SnapToTarget" true)
      (set `self.WeaponEquiped?` true))
    (:`B`
      (`self.K2_AttachToComponent` (`self.AI_WeaponRef`) (`self.Mesh`) "BackGunSocket" "SnapToTarget" "SnapToTarget" "SnapToTarget" true)
      (set `self.WeaponEquiped?` false)
      (set `self.IsEnemyFound?` false))))

(event `SpawnWeapon`
  ;[1 1 1] AI Toggle Weapon
  (bind _returnvalue (`|SpawnActorFromClass` (`self.EquipWeaponClass`) (`SceneComponent.K2_GetComponentToWorld` (`self.Sphere`)) "Undefined" "OverrideRootScale" null null))
  (bind _output_get (set `self.AI_WeaponRef` _returnvalue))
  (`self.K2_AttachToComponent` _output_get (`self.Mesh`) "BackGunSocket" "SnapToTarget" "SnapToTarget" "SnapToTarget" true)
  (`/Game/Levels/Level_1/Blueprints/Weapon_PickUp/BP_MasterWeaponPickUp.DestroyBox` (`self.AI_WeaponRef`)))

(event `self.PawnSensing.OnSeePawn`
  (params (Pawn :type "Pawn Object Reference"))
  (if (`self.ActorHasTag` Pawn "Player")
    (set `self.IsEnemyFound?` true)))

(event `ScanEnemy`
  (bind _arrow1 (`self.Arrow1`))
  (bind _returnvalue (`SceneComponent.K2_GetComponentLocation` _arrow1))
  ;[1 1 1] Check if enemy is in line of sight or not
  (bind (_outhit _returnvalue_2) (`KismetSystemLibrary.LineTraceSingle` _returnvalue (+ _returnvalue (* (`SceneComponent.GetForwardVector` _arrow1) 2000)) "TraceTypeQuery1" false (`|MakeArray` self :!type "Actor Object Reference")))
  (if _returnvalue_2
    (bind (_bblockinghit _binitialoverlap _time _distance _location _impactpoint _normal _impactnormal _physmat _hitactor) (`GameplayStatics.BreakHitResult` _outhit))
    (if (`KismetSystemLibrary.DoesImplementInterface` _hitactor "/Game/Levels/Level_1/Blueprints/Blueprint_Interface/BI_TakeDamage.BI_TakeDamage_C")
      (cast `/Game/Levels/Level_1/Blueprints/PlayerCharacter/BP_PlayerCharacter` _hitactor)
      (set `self.IsEnemyInSight` true)
      (else
        (set `self.IsEnemyInSight` false)))))

(event `self.AlertArea.OnComponentBeginOverlap`
  (params (OverlappedComponent :type "PrimitiveComponent Object Reference") (OtherActor :type "Actor Object Reference") (OtherComp :type "PrimitiveComponent Object Reference") (OtherBodyIndex :type Integer) (bFromSweep :type Boolean) (SweepResult :type "HitResult Structure (by ref)"))
  (if (not (`self.IsEnemyFound?`))
    (bind _asbp_master_ai (cast `/Game/Levels/Level_1/AI/BP_Master_AI` OtherActor))
    (if (`/Game/Levels/Level_1/AI/BP_Master_AI.IsDead?` _asbp_master_ai)
      (`KismetSystemLibrary.Delay` 1.0)
      (set `CharacterMovementComponent.MaxWalkSpeed` 150.0 (`self.CharacterMovement`))
      (`|AIMoveTo` self (`SceneComponent.K2_GetComponentLocation` (`Character.Mesh` _asbp_master_ai)) null 40.0
        (:`OnSuccess`
          _)
        (:`OnFail`
          _))
      (`KismetSystemLibrary.Delay` 4.0)
      (set `self.IsEnemyFound?` true)
      (set `CharacterMovementComponent.MaxWalkSpeed` 300.0 (`self.CharacterMovement`))
      (elif (`/Game/Levels/Level_1/AI/BP_Master_AI.IsEnemyFound?` _asbp_master_ai)
        (set `self.IsEnemyFound?` true)))))

(fn `UserConstructionScript`
  (bind _path (`self.Path`))
  (`SceneComponent.K2_DetachFromComponent` _path "KeepWorld" "KeepWorld" "KeepWorld" true)
  (set `self.MaxPathPoint` (`SplineComponent.GetNumberOfSplinePoints` _path)))